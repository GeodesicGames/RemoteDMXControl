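; DMX lighting fixture logic Blueprint that prepares a fixture's lights, materials and beam occlusion at BeginPlay.
; It creates dynamic beam, lens and light-function materials, then feeds gobo and color wheel disk textures and mask counts into all of them.
; Optional dynamic occlusion line-traces along the beam on a looping timer with randomized interval, setting the beam material's height from hit distance.
; Shadow casting and initial fixture state are also applied.
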(event `self.ReceiveBeginPlay`
  (bind _fixturebeammaterial (`self.FixtureBeamMaterial`))
  (bind _fixturelensmaterial (`self.FixtureLensMaterial`))
  (bind _fixturelightmaterial (`self.FixtureLightMaterial`))
  (bind _lightdynamicmaterial (`self.LightDynamicMaterial`))
  (bind _lightdynamicmaterial_2 (`self.LightDynamicMaterial`))
  (bind _fixturespotcomponent (`self.FixtureSpotComponent`))
  (bind _fixturepointlightcomponent (`self.FixturePointLightComponent`))
  (`|ExecutionSequence`
    (:`then_0`
      ;[1 1 1] Set cast shadow on light
      (`/Engine/EditorBlueprintResources/StandardMacros.IsValid` _fixturespotcomponent
        (:`Is Valid`
          (`LightComponentBase.SetCastShadows` _fixturespotcomponent (`self.Cast Shadow`)))))
    (:`then_1`
      (`/Engine/EditorBlueprintResources/StandardMacros.IsValid` _fixturepointlightcomponent
        (:`Is Valid`
          (`LightComponentBase.SetCastShadows` _fixturepointlightcomponent (`self.Cast Shadow`)))))
    (:`then_2`
      ;[1 1 1] Create dynamic beam material
      (`/Engine/EditorBlueprintResources/StandardMacros.IsValid` _fixturebeammaterial
        (:`Is Valid`
          (bind _returnvalue (`KismetMaterialLibrary.CreateDynamicMaterialInstance` _fixturebeammaterial))
          (bind _output_get (set `self.BeamDynamicMaterial` _returnvalue))
          (`self.AssignDynamicMaterialsToComponents` _output_get _fixturebeammaterial)
          (`KismetArrayLibrary.Array_Add` (`self.DynamicMaterialArray`) (`self.BeamDynamicMaterial`)))))
    (:`then_3`
      ;[1 1 1] Create dynamic Lens material
      (`/Engine/EditorBlueprintResources/StandardMacros.IsValid` _fixturelensmaterial
        (:`Is Valid`
          (bind _returnvalue_2 (`KismetMaterialLibrary.CreateDynamicMaterialInstance` _fixturelensmaterial))
          (bind _output_get_2 (set `self.LensDynamicMaterial` _returnvalue_2))
          (`self.AssignDynamicMaterialsToComponents` _output_get_2 _fixturelensmaterial)
          (`KismetArrayLibrary.Array_Add` (`self.DynamicMaterialArray`) (`self.LensDynamicMaterial`)))))
    (:`then_4`
      ;[1 1 1] Create dynamic Light function material
      (if (`KismetSystemLibrary.IsValid` _fixturelightmaterial)
        (bind _returnvalue_3 (`KismetMaterialLibrary.CreateDynamicMaterialInstance` _fixturelightmaterial))
        (bind _output_get_3 (set `self.LightDynamicMaterial` _returnvalue_3))
        (`KismetArrayLibrary.Array_Add` (`self.DynamicMaterialArray`) _output_get_3)))
    (:`then_5`
      ;[1 1 1] Set Point light
      (if (and (`KismetSystemLibrary.IsValid` (`self.FixturePointLightComponent`)) (`KismetSystemLibrary.IsValid` _lightdynamicmaterial_2))
        (`LightComponent.SetLightFunctionMaterial` (`self.FixturePointLightComponent`) _lightdynamicmaterial_2)))
    (:`then_6`
      ;[1 1 1] Set Spot light
      (if (and (`KismetSystemLibrary.IsValid` (`self.FixtureSpotComponent`)) (`KismetSystemLibrary.IsValid` _lightdynamicmaterial))
        (`LightComponent.SetLightFunctionMaterial` (`self.FixtureSpotComponent`) _lightdynamicmaterial)
        (else
          (`KismetSystemLibrary.PrintString` "INVALID"))))
    (:`then_7`
      ;[1 1 1] Create and assign Gobo Disk
      (`/Engine/EditorBlueprintResources/StandardMacros.IsValid` (`.DMXEffectTable_55_0666F58C45E899A178144F8C2A2A0174` (break `/DMXFixtures/Structs/Struct_ParameterData` (`self.GoboWheelData`)))
        (:`Is Valid`
          (bind (_clean _frosted) (`self.GetGoboDisk`))
          (for _array_element (`self.DynamicMaterialArray`)
            (`/Engine/EditorBlueprintResources/StandardMacros.IsValid` _array_element
              (:`Is Valid`
                (`MaterialInstanceDynamic.SetTextureParameterValue` _array_element "DMX Gobo Disk" _clean)
                (`MaterialInstanceDynamic.SetTextureParameterValue` _array_element "DMX Gobo Disk Frosted" _frosted)
                (`MaterialInstanceDynamic.SetScalarParameterValue` _array_element "DMX Gobo Num Mask" (`KismetMathLibrary.Conv_IntToDouble` (`KismetArrayLibrary.Array_Length` (`self.GoboMaskArray`))))))))))
    (:`then_8`
      ;[1 1 1] Create and assign color disk
      (`/Engine/EditorBlueprintResources/StandardMacros.IsValid` (`.DMXEffectTable_55_0666F58C45E899A178144F8C2A2A0174` (break `/DMXFixtures/Structs/Struct_ParameterData` (`self.ColorWheelData`)))
        (:`Is Valid`
          (bind _disk_clean (`self.GetColorDisk`))
          (for _array_element_2 (`self.DynamicMaterialArray`)
            (`/Engine/EditorBlueprintResources/StandardMacros.IsValid` _array_element_2
              (:`Is Valid`
                (`MaterialInstanceDynamic.SetTextureParameterValue` _array_element_2 "DMX Color Disk" _disk_clean)
                (`MaterialInstanceDynamic.SetScalarParameterValue` _array_element_2 "DMX Color Num Mask" (`KismetMathLibrary.Conv_IntToDouble` (`KismetArrayLibrary.Array_Length` (`self.ColorMaskArray`))))))))))
    (:`then_9`
      ;[1 1 1] Set Dynamic occlusion
      (if (and (`self.Use Dynamic Occlusion`) (`KismetSystemLibrary.IsValid` (`self.FixtureDynamicOcclusionComponent`)) (`KismetSystemLibrary.IsValid` (`self.BeamDynamicMaterial`)))
        (`KismetSystemLibrary.K2_SetTimerDelegate` (delegate `CustomEvent`) (`KismetMathLibrary.RandomFloatInRange` 0.1 0.3) true)))
    (:`then_10`
      (`self.SetInitialFixtureState`))))

(event `self.ReceiveTick`
  (params (DeltaSeconds :type "Float (single-precision)"))
  (`parent.ReceiveTick` DeltaSeconds))

(event `CustomEvent`
  (bind _beamdynamicmaterial (`self.BeamDynamicMaterial`))
  (bind _fixturedynamicocclusioncomponent (`self.FixtureDynamicOcclusionComponent`))
  (bind _returnvalue (`SceneComponent.K2_GetComponentLocation` _fixturedynamicocclusioncomponent))
  (bind _returnvalue_2 (* (`.SphereRadius` (`KismetSystemLibrary.GetComponentBounds` (`self.FixtureBeamComponent`))) 2.0))
  ;[1 1 1] Set Dynamic occlusion
  (bind (_outhit _returnvalue_3) (`KismetSystemLibrary.LineTraceSingle` :`Start` _returnvalue :`End` (+ _returnvalue (* (`SceneComponent.GetUpVector` _fixturedynamicocclusioncomponent) _returnvalue_2)) :`TraceChannel` "TraceTypeQuery1" :`bIgnoreSelf` false))
  (if _returnvalue_3
    (`MaterialInstanceDynamic.SetScalarParameterValue` _beamdynamicmaterial "DMX Dynamic Height" (`KismetMathLibrary.FClamp` (- 1.0 (/ (`.Distance` (`GameplayStatics.BreakHitResult` _outhit)) _returnvalue_2))))
    (else
      (`MaterialInstanceDynamic.SetScalarParameterValue` _beamdynamicmaterial "DMX Dynamic Height" 0.0))))

(fn `UserConstructionScript`
  (`parent.UserConstructionScript`))