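; BP_CustomStaticFixture is a DMX-controlled static light fixture supporting dimmer, strobe, zoom and color.
; On BeginPlay it assigns beam, lens and spotlight components, materials, parameter ranges and DMX function names to inherited fixture members, then calls the parent.
; It binds to the DMX subsystem's protocol-received event, reading normalized data and pushing all four parameters on each update.
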(event `self.ReceiveBeginPlay`
  ;[1 1 1] Initialize instance
  (set `self.FixtureParameterUsage` (make `/DMXFixtures/Structs/Struct_ParameterUsage` true true true true))
  (`self.AssignFixtureComponents`)
  (`self.AssignFixtureMaterials`)
  (`self.AssignFixtureParameters`)
  (`self.AssignFixtureMapping`)
  ;[1 1 1] Assign DMX event
  (add `DMXSubsystem.OnProtocolReceived` (subsystem `DMXSubsystem`) (delegate `CustomEvent_0`))
  (`parent.ReceiveBeginPlay`))

(event `CustomEvent_0`
  (params (Protocol :type "DMXProtocolName Structure") (Universe :type Integer) (DMXBuffer :type "Array of Byte (by ref)"))
  (bind ((`Dimmer_15_A4C47B3543C5B5010EA485997F88B873` _dimmer) (`Strobe_8_82140B434415AF152EBA5EBB2278FFFB` _strobe) (`Zoom_22_5DB7BD4048D4D706F36697A60CFFD0C0` _zoom) (`Color_26_958FA66B474C3BE74331DA9A64F7FB2D` _color)) (break `/DMXFixtures/Structs/Struct_DMXData` (`self.DMXCurrentNormalizedData`)))
  ;[1 1 1] Push new data when received
  (`self.GetDMXCurrentNormalizedData`)
  (`|ExecutionSequence`
    (:`then_0`
      (`self.PushDimmer` _dimmer))
    (:`then_1`
      (`self.PushStrobe` _strobe))
    (:`then_2`
      (`self.PushZoom` _zoom))
    (:`then_3`
      (`self.PushColor` _color))))

(fn `AssignFixtureComponents`
  (set `self.FixtureBeamComponent` (`self.Beam`))
  (set `self.FixtureLensComponent` (`self.Lens`))
  (set `self.FixtureSpotComponent` (`self.SpotLight`))
  (set `self.FixtureDynamicOcclusionComponent` (`self.Beam`)))

(fn `AssignFixtureMapping`
  (setmembers `/DMXFixtures/Structs/Struct_ParameterData` :`StructRef` (`self.DimmerData`) :`DMXFunctionName` (`self.DimmerFunctionName`))
  (setmembers `/DMXFixtures/Structs/Struct_ParameterData` :`StructRef` (`self.ZoomData`) :`DMXFunctionName` (`self.ZoomFunctionName`))
  (setmembers `/DMXFixtures/Structs/Struct_ParameterData` :`StructRef` (`self.StrobeData`) :`DMXFunctionName` (`self.StrobeFunctionName`))
  (setmembers `/DMXFixtures/Structs/Struct_ColorParameterData` :`StructRef` (`self.ColorData`) :`DMXFunctionName_1` (`self.ColorChannelFunctionName1`) :`DMXFunctionName_2` (`self.ColorChannelFunctionName2`) :`DMXFunctionName_3` (`self.ColorChannelFunctionName3`)))

(fn `AssignFixtureMaterials`
  (set `self.FixtureBeamMaterial` "/DMXFixtures/Masters/M_BeamStatic_Master.M_BeamStatic_Master")
  (set `self.FixtureLensMaterial` "/DMXFixtures/Masters/M_Lens_Static_Master.M_Lens_Static_Master")
  (set `self.FixtureLightMaterial` "/DMXFixtures/Masters/M_Light_Master.M_Light_Master"))

(fn `AssignFixtureParameters`
  (set `self.FixtureIntensityMax` (`self.IntensityMax (Lumens)`))
  (`self.SetParameterRange` (`self.ZoomData`) (`self.Zoom Min (Deg)`) (`self.Zoom Max (Deg)`))
  (`self.SetParameterEffectTable` (`self.StrobeData`) (`self.StrobeEffectTable`)))

(fn `UserConstructionScript`)